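; BP_ManageableObjectsManager is a registry that keeps a list of manageable objects and looks them up by gameplay tag.
; Two events add objects to and remove them from ManageablesList.
; GetAllManageablesWithTag clears a return array, scans the list and collects every entry whose ManageableTag container holds an exact match for the given tag.
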(event Custom|AddNewManageable
  (params (NewManageable :type Manageable%20Component%20Object%20Reference))
  (Utilities|Array|Add (Variables|Default|GetManageablesList) NewManageable))

(event Custom|RemoveManageable
  (params (ManageanleToRemove :type Manageable%20Component%20Object%20Reference))
  (Utilities|Array|RemoveItem (Variables|Default|GetManageablesList) ManageanleToRemove))

(fn GetAllManageableswithTag
  (params (GameplayTag :type Gameplay%20Tag%20Structure))
  (bind _returnarray (Variables|Default|GetReturnArray))
  (Utilities|Array|Clear (Variables|Default|GetReturnArray))
  (for _array_element (Variables|Default|GetManageablesList)
    (if (GameplayTags|HasTag (Variables|/Game/Systems/Components/ManageableComponent.ManageableComponent_C|GetManageableTag _array_element) GameplayTag true)
      (Utilities|Array|Add _returnarray _array_element)))
  (return _returnarray))
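; Pad is a programmable Blueprint that acts as a socket holding one connected pickable block at a time.
; ConnectBlock stores the incoming Pickable as CurrentPickable, and DisconnectBlock clears it.
; CanConnect allows a connection only when the pad is empty and the Pickable's owner has a component of any class listed in StickableComponents.
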(event Custom|ConnectBlock
  (params (Pickable :type Pickable%20Component%20Object%20Reference))
  (Variables|Default|SetCurrentPickable Pickable))

(event Custom|DisconnectBlock
  (Variables|Default|SetCurrentPickable 0))

(fn ConstructionScript)

(fn CanConnect
  (params (Pickable :type Pickable%20Component%20Object%20Reference))
  (for _array_element (Variables|PadDefault|GetStickableComponents)
    (Utilities|IsValid (Actor|GetComponentbyClass (Components|GetOwner Pickable) _array_element)
      (:Is%20Valid
        (LocalVariables|SetHasStickableComp? true))))
  (return (and (not (Utilities|IsValid (Variables|Default|GetCurrentPickable))) (LocalVariables|GetHasStickableComp?))))
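; Programable actor that turns blocks on its pads into a rule that changes tagged objects in the game.
; It registers with each pad on BeginPlay, and on refresh reads their blocks as tag, operation type and component.
; A complete code adds that component to all manageables with the tag via the manageable objects manager.
; When the code becomes incomplete, it removes the previous code's component; only one operation type is handled.
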(event Custom|RefreshProgramable
  (bind _currentcode (Variables|Pads|GetCurrentCode))
  ;[0 0 0] Refresh programable and execute new code
  (Variables|Pads|SetOldCode _currentcode)
  (Utilities|Array|Clear _currentcode)
  (for _array_element (Variables|Pads|GetPads)
    (Utilities|Array|Add (Variables|Pads|GetCurrentCode) (Variables|/Game/Blueprints/Programables/ProgramablePad.ProgramablePad_C|GetCurrentBlock _array_element)))
  (if (Utilities|Array|ContainsItem (Variables|Pads|GetCurrentCode) 0)
    (if (not (Utilities|Array|ContainsItem (Variables|Pads|GetOldCode) 0))
      (CallFunction|RevertOldCode))
    (else
      (CallFunction|ExecuteNewCode))))

(event Custom|RevertOldCode
  (bind _oldcode (Variables|Pads|GetOldCode))
  ;[0 0 0] Revert old code
  (if (not (Utilities|Array|IsEmpty _oldcode))
    (bind _returnarray (Default|GetAllManageableswithTag (Subsystems|GetBPManageableObjectsManager) (Variables|/Game/Systems/Components/BlockComponent.BlockComponent_C|GetGameplayTag (Utilities|Array|Get(acopy) _oldcode))))
    (if (Utilities|Enum|Equal(Enum) (Variables|/Game/Systems/Components/BlockComponent.BlockComponent_C|GetType (Utilities|Array|Get(acopy) (Variables|Pads|GetOldCode) 1)) "NewEnumerator1")
      (for _array_element _returnarray
        (Default|RemoveComponent _array_element (Variables|/Game/Systems/Components/BlockComponent.BlockComponent_C|GetComponent (Utilities|Array|Get(acopy) (Variables|Pads|GetOldCode) 2)))))))

(event Custom|ExecuteNewCode
  ;[0 0 0] Execute current code
  (bind _returnarray (Default|GetAllManageableswithTag (Subsystems|GetBPManageableObjectsManager) (Variables|/Game/Systems/Components/BlockComponent.BlockComponent_C|GetGameplayTag (Utilities|Array|Get(acopy) (Variables|Pads|GetCurrentCode)))))
  (if (Utilities|Enum|Equal(Enum) (Variables|/Game/Systems/Components/BlockComponent.BlockComponent_C|GetType (Utilities|Array|Get(acopy) (Variables|Pads|GetCurrentCode) 1)) "NewEnumerator1")
    (for _array_element _returnarray
      (Default|AddNewComponent _array_element (Variables|/Game/Systems/Components/BlockComponent.BlockComponent_C|GetComponent (Utilities|Array|Get(acopy) (Variables|Pads|GetCurrentCode) 2))))))

(event EventBeginPlay
  ;[0 0 0] Add programable to pads
  (for _array_element (Variables|Pads|GetPads)
    (Default|AddProgramable _array_element self)))

(fn ConstructionScript)